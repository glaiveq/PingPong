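; BP_Goals is a goal trigger that adds a point to one of two scores in a ping pong game.
; On BeginPlay it caches the first player controller as a BP_PingPongPlayerController.
; When anything begins overlapping GoalCollision, the FirstPlayerScored flag selects whether Score1 or Score2 on that controller goes up by one.
; The overlap does not filter the other actor or reset play.
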(event OnComponentBeginOverlap(GoalCollision)
  (params (OverlappedComponent :type Primitive%20Component%20Object%20Reference) (OtherActor :type Actor%20Object%20Reference) (OtherComp :type Primitive%20Component%20Object%20Reference) (OtherBodyIndex :type Integer) (bFromSweep :type Boolean) (SweepResult :type Hit%20Result%20Structure%20%28by%20ref%29))
  (bind _playercontrollerref (Variables|Default|GetPlayerControllerRef))
  (if (Variables|Default|GetbFirstPlayerScored?)
    (Utilities|IsValid _playercontrollerref
      (:Is%20Valid
        (Variables|/Game/Blueprints/Controller/BP_PingPongPlayerController.BP_PingPongPlayerController_C|SetScore1 _playercontrollerref (+ (Variables|/Game/Blueprints/Controller/BP_PingPongPlayerController.BP_PingPongPlayerController_C|GetScore1 _playercontrollerref) 1))))
    (else
      (Utilities|IsValid _playercontrollerref
        (:Is%20Valid
          (Variables|/Game/Blueprints/Controller/BP_PingPongPlayerController.BP_PingPongPlayerController_C|SetScore2 _playercontrollerref (+ (Variables|/Game/Blueprints/Controller/BP_PingPongPlayerController.BP_PingPongPlayerController_C|GetScore2 _playercontrollerref) 1)))))))

(event EventBeginPlay
  (bind _asbp_ping_pong_player_controller (Utilities|Casting|CastToBP_PingPongPlayerController (Game|GetPlayerController 0)))
  (Variables|Default|SetPlayerControllerRef _asbp_ping_pong_player_controller))

(fn ConstructionScript)